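; BlocBase_BP is a block actor, apparently a base class, that sits on a grid with 100-unit cells.
; SetLocation stores the grid coordinate in Location and moves the actor to that value multiplied by 100 on each axis, without sweeping.
; The construction script reapplies the stored Location, so placement follows the variable, and the event graph holds no active logic.
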(fn `SetLocation`
  (params (Location :type "IntVector Structure"))
  (bind _output_get (set `self.Location` Location))
  (bind (_x _y _z) (break `IntVector` _output_get))
  (`self.K2_SetActorLocation` (`KismetMathLibrary.MakeVector` (`KismetMathLibrary.Conv_IntToDouble` (* _x 100)) (`KismetMathLibrary.Conv_IntToDouble` (* _y 100)) (`KismetMathLibrary.Conv_IntToDouble` (* _z 100)))))

(fn `UserConstructionScript`
  (`self.SetLocation` (`self.Location`)))