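; UpDownBlock_BP is a block actor that bobs up and down in an endless loop between its starting location and 50 units above it.
; After a configurable Delay on BeginPlay, Restart uses a FlipFlop to alternately play a Timeline forward and in reverse.
; The Timeline's track drives a vector lerp that sets the actor's location without sweeping, and its Finished output calls Restart again.
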(event `self.ReceiveBeginPlay`
  (set `self.DefaultLoc` (`self.K2_GetActorLocation`))
  (`KismetSystemLibrary.Delay` (`self.Delay`))
  (`self.Restart`))

(event `Restart`
  (bind _defaultloc (`self.DefaultLoc`))
  (`/Engine/EditorBlueprintResources/StandardMacros.FlipFlop`
    (:`A`
      (bind (_direction _newtrack_0) (`Timeline|Timeline` :!via `PlayFromStart` :!label _label)
        (:`Update`
          (`self.K2_SetActorLocation` (`KismetMathLibrary.VLerp` _defaultloc (+ _defaultloc (0.0 0.0 50.0)) _newtrack_0)))
        (:`Finished`
          (`self.Restart`))))
    (:`B`
      (goto _label :!via `ReverseFromEnd`))))

(fn `UserConstructionScript`)