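; Chunk actor that builds one tile of noise-driven block terrain in its construction script, using the world reference's settings.
; Each column gets a height-placed cube with a material from temperature and biome noise, plus water at height -1 or ramp and edge meshes where one or two neighbors are higher.
; Blocks collect in a location-keyed map, then spawn into HISM components created lazily per mesh and material pair.
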(fn `Add Ramp To Terrain`
  (params (UpperBlockLocation :type "IntVector Structure") (HigherNeighbors :type "Array of IntVector Structure") (UpperBlockMaterial :type "Material Object Reference"))
  (bind _upperblocklocation (`local.UpperBlockLocation`))
  (bind (_ramprotation _edgelocationdifference) (`/Game/World/Chunk_FL.GetRampRotation` (`/Game/World/Chunk_ML.SubstractIntVectors` _upperblocklocation (`|GetArrayItem` (`local.HigherNeighbors`)))))
  (`self.AddInstance` (make `/Game/World/BlockData_STRUCT` "/Game/World/Models/Ramp_SM.Ramp_SM" UpperBlockMaterial) _upperblocklocation _ramprotation)
  (`self.AddInstance` (make `/Game/World/BlockData_STRUCT` "/Game/World/Models/Edge_SM.Edge_SM" UpperBlockMaterial) (`/Game/World/Chunk_ML.AddIntVectors` _edgelocationdifference (`local.UpperBlockLocation`)) _ramprotation false))

(fn `AddCubeToTerrain`
  (params (BlockLocation :type "IntVector Structure"))
  (returns (BlockMaterial :type "Material Object Reference"))
  (bind (_x _y) (break `IntVector` BlockLocation))
  (bind _worldref (`self.WorldRef`))
  (bind (_blocklocation_x _blocklocation_y) (break `IntVector` (`local.BlockLocation`)))
  (bind _temperature (`/Game/World/Chunk_FL.GetBlockTemperature` (`/Game/World/World_BP.TemperatureNoise` _worldref) _x _y))
  (bind _biome (`/Game/World/Chunk_FL.GetBlockBiome` (`/Game/World/World_BP.BiomeNoise` _worldref) _blocklocation_x _blocklocation_y _temperature))
  (bind _blocksmaterial (`/Game/World/Biome/Biome_BP.BlocksMaterial` _biome))
  (`self.AddInstance` (make `/Game/World/BlockData_STRUCT` "/Game/World/Models/Cube_SM.Cube_SM" _blocksmaterial) (`local.BlockLocation`))
  (return _blocksmaterial))

(fn `AddInstance`
  (params (BlockData :type "/Game/World/BlockData_STRUCT Structure") (InstanceLocation :type "IntVector Structure") (InstanceRotation :type "Rotator Structure") (ReplaceExistingInstance :type Boolean :default true))
  (locals (HISM :type "HierarchicalInstancedStaticMeshComponent Object Reference"))
  (if ReplaceExistingInstance
    (`BlueprintMapLibrary.Map_Add` (`self.Instances`) (`local.InstanceLocation`) (make `/Game/World/InstanceData_STRUCT` (`local.BlockData`) (`local.InstanceRotation`)))
    (else
      (bind _keys (`BlueprintMapLibrary.Map_Keys` (`self.Instances`)))
      (if (not (`KismetArrayLibrary.Array_Contains` _keys (`local.InstanceLocation`)))
        (`BlueprintMapLibrary.Map_Add` (`self.Instances`) (`local.InstanceLocation`) (make `/Game/World/InstanceData_STRUCT` (`local.BlockData`) (`local.InstanceRotation`)))))))

(fn `AddOuterEdgeToTerrain`
  (params (UpperBlockLocation :type "IntVector Structure") (HigherNeighbors :type "Array of IntVector Structure") (UpperBlockMaterial :type "Material Object Reference"))
  (bind (_ramprotation _edgelocationdifference) (`/Game/World/Chunk_FL.GetOuterEdgeRotation` (`/Game/World/Chunk_ML.AddIntVectors` (`/Game/World/Chunk_ML.SubstractIntVectors` UpperBlockLocation (`|GetArrayItem` HigherNeighbors)) (`/Game/World/Chunk_ML.SubstractIntVectors` UpperBlockLocation (`|GetArrayItem` HigherNeighbors 1)))))
  (`self.AddInstance` (make `/Game/World/BlockData_STRUCT` "/Game/World/Models/OuterEdge_SM.OuterEdge_SM" UpperBlockMaterial) (`local.UpperBlockLocation`) _ramprotation)
  (`self.AddInstance` (make `/Game/World/BlockData_STRUCT` "/Game/World/Models/Edge_SM.Edge_SM" (`local.UpperBlockMaterial`)) (`/Game/World/Chunk_ML.AddIntVectors` _edgelocationdifference (`local.UpperBlockLocation`)) _ramprotation false))

(fn `AddUpperBlockToTerrain`
  (params (BlockLocation :type "IntVector Structure") (BlockMaterial :type "Material Object Reference"))
  (locals (UpperBlockLocation :type "IntVector Structure") (HigherNeighbors :type "Array of IntVector Structure"))
  (bind (_x _y _z) (break `IntVector` BlockLocation))
  (set `local.UpperBlockLocation` (make `IntVector` _x _y (+ _z 1)))
  (bind _higher_neighbors (`/Game/World/Chunk_FL.GetHigherNeighbors` (`local.BlockLocation`) (`/Game/World/World_BP.HeightNoise` (`self.WorldRef`))))
  (bind _output_get (set `local.HigherNeighbors` _higher_neighbors))
  (switch `int` (`KismetArrayLibrary.Array_Length` _output_get)
    (:`1`
      (`self.Add Ramp To Terrain` (`local.UpperBlockLocation`) (`local.HigherNeighbors`) (`local.BlockMaterial`)))
    (:`2`
      (`self.AddOuterEdgeToTerrain` (`local.UpperBlockLocation`) (`local.HigherNeighbors`) (`local.BlockMaterial`)))))

(fn `AddWaterToTerrain`
  (params (BlockPosition :type "IntVector Structure"))
  (bind (_x _y _z) (break `IntVector` BlockPosition))
  (`self.AddInstance` (make `/Game/World/BlockData_STRUCT` "/Game/World/Models/Water_SM.Water_SM" "/Game/World/Models/Water_MAT.Water_MAT") (make `IntVector` _x _y (+ _z 1))))

(fn `GetOrCreateHISM`
  (params (BlockData :type "/Game/World/BlockData_STRUCT Structure (by ref)"))
  (returns (HISM :type "HierarchicalInstancedStaticMeshComponent Object Reference"))
  (locals (Result :type "HierarchicalInstancedStaticMeshComponent Object Reference"))
  (bind _blockdata (`local.BlockData`))
  (bind (_staticmesh _material) (break `/Game/World/BlockData_STRUCT` _blockdata))
  (bind (_value _returnvalue) (`BlueprintMapLibrary.Map_Find` (`self.HISMs`) BlockData))
  (if _returnvalue
    (return _value)
    (else
      (bind _returnvalue_2 (`AddComponent|NODE_AddHierarchicalInstancedStaticMeshComponent-3`))
      (`BlueprintMapLibrary.Map_Add` (`self.HISMs`) _blockdata _returnvalue_2)
      (`StaticMeshComponent.SetStaticMesh` _returnvalue_2 _staticmesh)
      (`PrimitiveComponent.SetMaterial` _returnvalue_2 0 _material)
      (return _returnvalue_2))))

(fn `SpawnInstance`
  (params (InstanceData :type "/Game/World/InstanceData_STRUCT Structure (by ref)") (Location :type "IntVector Structure"))
  (bind (_blockdata _instancerotation) (break `/Game/World/InstanceData_STRUCT` InstanceData))
  (bind _hism (`self.GetOrCreateHISM` _blockdata))
  (`InstancedStaticMeshComponent.AddInstance` _hism (`KismetMathLibrary.MakeRelativeTransform` (`KismetMathLibrary.MakeTransform` (`/Game/World/Chunk_ML.Location To Vector` Location) _instancerotation) (`self.GetTransform`)) false))

(fn `SpawnTerrain`
  (locals (`Block X` :type Integer) (`Block Y` :type Integer))
  (bind _instances (`self.Instances`))
  (bind (_chunklocation_x _chunklocation_y _chunklocation_z) (break `IntVector` (`self.ChunkLocation`)))
  (bind _returnvalue (+ (`local.Block X`) _chunklocation_x))
  (bind _returnvalue_2 (+ (`local.Block Y`) _chunklocation_y))
  (for _index (range (`/Game/World/World_BP.ChunkSize` (`self.WorldRef`)))
    (set `local.Block X` _index)
    (for _index_2 (range (`/Game/World/World_BP.ChunkSize` (`self.WorldRef`)))
      (set `local.Block Y` _index_2)
      (bind _bloc_z (`/Game/World/Chunk_FL.GetBlockHeight` (`/Game/World/World_BP.HeightNoise` (`self.WorldRef`)) _returnvalue _returnvalue_2))
      (bind _intvector (make `IntVector` _returnvalue _returnvalue_2 (+ _bloc_z _chunklocation_z)))
      (bind _blockmaterial (`self.AddCubeToTerrain` _intvector))
      (if (== _bloc_z -1)
        (`self.AddWaterToTerrain` _intvector)
        (else
          (`self.AddUpperBlockToTerrain` _intvector _blockmaterial)))))
  (bind _keys (`BlueprintMapLibrary.Map_Keys` _instances))
  (for _array_element _keys
    (`self.SpawnInstance` (`BlueprintMapLibrary.Map_Find` _instances _array_element) _array_element)))

(fn `UserConstructionScript`
  (`self.SpawnTerrain`))