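; Terrain chunk actor that builds a block grid from seeded FastNoise heights in its construction script, using instanced static meshes.
; Each floor cell checks its four neighbors for higher ground to add ramps, outer edges or fill blocks.
; Edge pieces are recorded in a map so later placements can remove overlapping ones.
; BeginPlay scatters a few Tree_BP actors within the chunk, which are destroyed along with it.
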(event `self.ReceiveBeginPlay`
  (bind (_location_x _location_y _location_z) (break `IntVector` (`self.Location`)))
  (bind _chunksize (`self.ChunkSize`))
  (bind _returnvalue (`KismetMathLibrary.RandomIntegerInRange` _location_y (+ _location_y _chunksize)))
  (bind _returnvalue_2 (`KismetMathLibrary.RandomIntegerInRange` _location_x (+ _location_x _chunksize)))
  (for _ (range 3)
    (bind _returnvalue_3 (`|SpawnActorFromClass` "/Game/Blocs/Tree_BP.Tree_BP_C" (`KismetMathLibrary.MakeTransform` (0.0 0.0 0.0)) "Undefined" "MultiplyWithRoot" null (make `IntVector` _returnvalue_2 _returnvalue (+ (`self.GetZHeight` _returnvalue_2 _returnvalue _location_z) 1)) null))
    (`KismetArrayLibrary.Array_Add` (`self.SpawnedActors`) _returnvalue_3)))

(event `self.ReceiveDestroyed`
  (for _array_element (`self.SpawnedActors`)
    (`self.K2_DestroyActor` _array_element)))

(fn `Check Neighbors`
  (params (`Bloc location` :type "IntVector Structure"))
  (returns (`Higher Neighbors` :type "Array of IntVector Structure"))
  (locals (`Higher Neighbor` :type "Array of IntVector Structure") (ZHeight :type Integer :default 0))
  (bind (_bloc_location_x _bloc_location_y _bloc_location_z) (break `IntVector` (`local.Bloc location`)))
  (bind (_bloc_location_x_2 _bloc_location_y_2 _bloc_location_z_2) (break `IntVector` (`local.Bloc location`)))
  (bind (_bloc_location_x_3 _bloc_location_y_3 _bloc_location_z_3) (break `IntVector` (`local.Bloc location`)))
  (bind (_bloc_location_x_4 _bloc_location_y_4 _bloc_location_z_4) (break `IntVector` (`local.Bloc location`)))
  (bind _returnvalue (- _bloc_location_x_2 1))
  (bind _returnvalue_2 (+ _bloc_location_x_3 1))
  (bind _returnvalue_3 (- _bloc_location_y_4 1))
  (bind _returnvalue_4 (+ _bloc_location_y 1))
  (set `local.ZHeight` (`self.GetZHeight` `Bloc location_X` `Bloc location_Y` `Bloc location_Z`))
  (`|ExecutionSequence`
    (:`then_0`
      ;[1 1 1] X = -1
      (if (> (`self.GetZHeight` _returnvalue _bloc_location_y_2 _bloc_location_z_2) (`local.ZHeight`))
        (`KismetArrayLibrary.Array_Add` (`local.Higher Neighbor`) (make `IntVector` _returnvalue _bloc_location_y_2 _bloc_location_z_2))))
    (:`then_1`
      ;[1 1 1] X = +1
      (if (> (`self.GetZHeight` _returnvalue_2 _bloc_location_y_3 _bloc_location_z_3) (`local.ZHeight`))
        (`KismetArrayLibrary.Array_Add` (`local.Higher Neighbor`) (make `IntVector` _returnvalue_2 _bloc_location_y_3 _bloc_location_z_3))))
    (:`then_2`
      ;[1 1 1] Y = -1
      (if (> (`self.GetZHeight` _bloc_location_x_4 _returnvalue_3 _bloc_location_z_4) (`local.ZHeight`))
        (`KismetArrayLibrary.Array_Add` (`local.Higher Neighbor`) (make `IntVector` _bloc_location_x_4 _returnvalue_3 _bloc_location_z_4))))
    (:`then_3`
      ;[1 1 1] Y = +1
      (if (> (`self.GetZHeight` _bloc_location_x _returnvalue_4 _bloc_location_z) (`local.ZHeight`))
        (`KismetArrayLibrary.Array_Add` (`local.Higher Neighbor`) (make `IntVector` _bloc_location_x _returnvalue_4 _bloc_location_z))))
    (:`then_4`
      (return (`local.Higher Neighbor`)))))

(fn `Get Upper OuterEdge Rotation`
  (params (Difference :type "IntVector Structure"))
  (returns (`Z Rotation` :type Integer))
  (bind _returnvalue (== Difference_Y -1))
  (if (== Difference_X -1)
    (if _returnvalue
      (return 2)
      (else
        (return 1)))
    (elif _returnvalue
      (return 3)
      (else
        (return 0)))))

(fn `Get Upper Ramp Rotation`
  (params (Difference :type "IntVector Structure"))
  (returns (`Z Rotation` :type Integer))
  (switch `int` Difference_X
    (:`-1`
      (return 1))
    (:`0`
      (switch `int` Difference_Y
        (:`-1`
          (return 2))
        (:`0`
          _)
        (:`1`
          _))
      (return 0))
    (:`1`
      (return 3))))

(fn `GetZHeight`
  (params (X :type Integer) (Y :type Integer) (Z :type Integer))
  (returns (`Z Location` :type Integer))
  (return (`KismetMathLibrary.Round` (`FastNoiseWrapper.GetNoise3D` (`self.FastNoiseWrapper`) (`self.LocationToCoordinates` X) (`self.LocationToCoordinates` Y) (`self.LocationToCoordinates` Z)))))

(fn `Spawn Edge`
  (params (BlocLocation :type "IntVector Structure") (`Bloc Z Rotation` :type Integer))
  (locals (EdgeLocation :type "IntVector Structure"))
  (switch `int` `Bloc Z Rotation`
    (:`0`
      (set `local.EdgeLocation` (`self.AddIntVector` (`local.BlocLocation`) (make `IntVector` 1))))
    (:`1`
      (set `local.EdgeLocation` (`self.AddIntVector` (`local.BlocLocation`) (make `IntVector` 0 1))))
    (:`2`
      (set `local.EdgeLocation` (`self.SubstracIntVector` (`local.BlocLocation`) (make `IntVector` 1))))
    (:`3`
      (set `local.EdgeLocation` (`self.SubstracIntVector` (`local.BlocLocation`) (make `IntVector` 0 1)))))
  (bind _instance (`self.Spawn Instance` (`self.Edges`) (`local.EdgeLocation`) (`local.Bloc Z Rotation`)))
  (`BlueprintMapLibrary.Map_Add` (`self.EdgesInstances`) (struct) _instance))

(fn `Spawn Instance`
  (params (`Instanced Static Mesh` :type "InstancedStaticMeshComponent Object Reference") (Location :type "IntVector Structure") (`Z Rotation` :type Integer))
  (returns (Instance :type Integer))
  (bind (_x _y _z) (break `IntVector` Location))
  (bind (_value _returnvalue) (`BlueprintMapLibrary.Map_Find` (`self.EdgesInstances`) Location))
  (if _returnvalue
    (`InstancedStaticMeshComponent.RemoveInstance` (`self.Edges`) _value))
  (bind _returnvalue_2 (`InstancedStaticMeshComponent.AddInstance` (`local.Instanced Static Mesh`) (`KismetMathLibrary.MakeTransform` (`KismetMathLibrary.MakeVector` (`self.LocationToCoordinates` _x) (`self.LocationToCoordinates` _y) (`self.LocationToCoordinates` _z)) (`KismetMathLibrary.MakeRotator` 0.0 0.0 (`KismetMathLibrary.Conv_IntToDouble` (* `Z Rotation` 90)))) false))
  (return _returnvalue_2))

(fn `Spawn Outer Edge`
  (params (`Bloc Location` :type "IntVector Structure (by ref)") (FirstNeighborLocation :type "IntVector Structure") (SecondNeighborLocation :type "IntVector Structure"))
  (bind _z_rotation (`self.Get Upper OuterEdge Rotation` (`self.AddIntVector` (`self.SubstracIntVector` `Bloc Location` FirstNeighborLocation) (`self.SubstracIntVector` `Bloc Location` SecondNeighborLocation))))
  (`self.Spawn Instance` (`self.Outer Edges`) `Bloc Location` _z_rotation)
  (`self.Spawn Edge` (`local.Bloc Location`) _z_rotation))

(fn `Spawn Ramp`
  (params (`Bloc Location` :type "IntVector Structure (by ref)") (`Neighbor Location` :type "IntVector Structure"))
  (bind _z_rotation (`self.Get Upper Ramp Rotation` (`self.SubstracIntVector` `Bloc Location` `Neighbor Location`)))
  (`self.Spawn Instance` (`self.Ramps`) `Bloc Location` _z_rotation)
  (`self.Spawn Edge` `Bloc Location` _z_rotation))

(fn `Spawn Three Neighbors`
  (params (`Bloc Location` :type "IntVector Structure") (`First Neighbor` :type "IntVector Structure") (`Second Neighbor` :type "IntVector Structure") (`Third Neighbor` :type "IntVector Structure"))
  (bind (_bloc_location_x _bloc_location_y _bloc_location_z) (break `IntVector` (`local.Bloc Location`)))
  (bind _bloc_location (`local.Bloc Location`))
  (bind (_x _y) (break `IntVector` (`self.AddIntVector` (`self.AddIntVector` (`self.SubstracIntVector` `Bloc Location` `First Neighbor`) (`self.SubstracIntVector` `Bloc Location` `Second Neighbor`)) (`self.SubstracIntVector` `Bloc Location` `Third Neighbor`))))
  (bind _intvector (make `IntVector` (- 0 _x) (- 0 _y) _bloc_location_z))
  (bind (_result_x _result_y) (break `IntVector` (`self.SubstracIntVector` _bloc_location _intvector)))
  (`self.Spawn Instance` (`self.Floor`) (`local.Bloc Location`))
  (`self.Spawn Instance` (`self.Ramps`) (make `IntVector` _result_x _result_y (`.Z` (break `IntVector` _bloc_location))) (`self.Get Upper Ramp Rotation` (`self.SubstracIntVector` (make `IntVector` 0) _intvector))))

(fn `Spawn Upper Bloc`
  (params (HigherNeighbors :type "Array of IntVector Structure") (`Bloc Location` :type "IntVector Structure"))
  (switch `int` (`KismetArrayLibrary.Array_Length` HigherNeighbors)
    (:`1`
      (`self.Spawn Ramp` `Bloc Location` (`|GetArrayItem` HigherNeighbors)))
    (:`2`
      (`self.Spawn Outer Edge` `Bloc Location` (`|GetArrayItem` HigherNeighbors) (`|GetArrayItem` HigherNeighbors 1)))
    (:`3`
      (`self.Spawn Three Neighbors` `Bloc Location` (`|GetArrayItem` HigherNeighbors) (`|GetArrayItem` HigherNeighbors 1) (`|GetArrayItem` HigherNeighbors 2)))))

(fn `SpawnBlocs`
  (bind _chunksize (`self.ChunkSize`))
  (bind (_x _y _z) (break `IntVector` (`self.Location`)))
  (for _index (range (+ _chunksize 1))
    (for _index_2 (range (+ _chunksize 1))
      (bind _returnvalue (+ _index _x))
      (bind _returnvalue_2 (+ _index_2 _y))
      (bind _intvector (make `IntVector` _returnvalue _returnvalue_2 (`self.GetZHeight` _returnvalue _returnvalue_2 _z)))
      (`self.Spawn Instance` (`self.Floor`) _intvector)
      (bind _higher_neighbors (`self.Check Neighbors` (make `IntVector` _returnvalue _returnvalue_2 _z)))
      (`self.Spawn Upper Bloc` _higher_neighbors (`self.AddIntVector` _intvector (make `IntVector` 0 0 1))))))

(fn `UserConstructionScript`
  (bind _returnvalue (`|GenericCreateObject` "/Script/FastNoiseGenerator.FastNoiseWrapper"))
  (bind _output_get (set `self.FastNoiseWrapper` _returnvalue))
  (`FastNoiseWrapper.SetupFastNoise` _output_get "Simplex" (`self.Seed`) (`self.Frequency`) "Quintic" "FBM" 3 2.0 0.5 0.45 "Euclidean" "CellValue")
  (`self.SpawnBlocs`))