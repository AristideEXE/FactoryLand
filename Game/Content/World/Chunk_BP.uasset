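; Terrain chunk Blueprint that builds a grid of block instances with noise-driven heights in its construction script.
; It creates a FastNoise wrapper, then loops over ChunkSize in X and Y, offsetting each cell by Location in block units.
; Each cell samples 3D noise, rounds the raw value before scaling by block size for stepped heights, and adds a local-space instance to Floor.
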(fn `UserConstructionScript`
  (bind _chunksize (`self.ChunkSize`))
  (bind _singleblocsize (`self.SingleBlocSize`))
  (bind (_x _y _z) (break `IntVector` (`self.Location`)))
  (bind _returnvalue (`|GenericCreateObject` "/Script/FastNoiseGenerator.FastNoiseWrapper"))
  (bind _output_get (set `self.FastNoiseWrapper` _returnvalue))
  (`FastNoiseWrapper.SetupFastNoise` _output_get "Simplex" 1337 0.0003 "Quintic" "FBM" 3 2.0 0.5 0.45 "Euclidean" "CellValue")
  (for _index (range (+ _chunksize 1))
    (for _index_2 (range (+ _chunksize 1))
      (bind _returnvalue_2 (`KismetMathLibrary.Conv_IntToDouble` (+ (* _x _singleblocsize) (* _index _singleblocsize))))
      (bind _returnvalue_3 (`KismetMathLibrary.Conv_IntToDouble` (+ (* _y _singleblocsize) (* _index_2 _singleblocsize))))
      (`InstancedStaticMeshComponent.AddInstance` (`self.Floor`) (`KismetMathLibrary.MakeTransform` (`KismetMathLibrary.MakeVector` _returnvalue_2 _returnvalue_3 (`KismetMathLibrary.Conv_IntToDouble` (* (`KismetMathLibrary.Round` (`FastNoiseWrapper.GetNoise3D` (`self.FastNoiseWrapper`) _returnvalue_2 _returnvalue_3 (`KismetMathLibrary.Conv_IntToDouble` (* _z _singleblocsize)))) (`self.SingleBlocSize`))))) false))))